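; BP_Pistol is a modular pistol that assembles its visual model from a WeaponParts array when play begins.
; BeginPlay validity-checks array entries by fixed index and assigns them as static meshes to the frame, trigger, barrel, magazine and slider socket components.
; Trigger and barrel are only set when the frame mesh is valid, while magazine and slider are set independently.
; The construction script only calls its parent.
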(event Collision|EventActorBeginOverlap
  (params (OtherActor :type Actor%20Object%20Reference))
  (|CallParentFunction OtherActor) ; This node is disabled and will not be called.\nDrag off pins to build functionality.
)

(event EventTick
  (params (DeltaSeconds :type Float%20%28single-precision%29))
  (|CallParentFunction DeltaSeconds) ; This node is disabled and will not be called.\nDrag off pins to build functionality.
)

(event EventBeginPlay
  (bind _weapon_parts (Variables|Default|Getweapon%20parts))
  (bind _weapon_parts_2 (Variables|Default|Getweapon%20parts))
  (bind _weapon_parts_3 (Variables|Default|Getweapon%20parts))
  (bind _weapon_parts_4 (Variables|Default|Getweapon%20parts))
  (bind _weapon_parts_5 (Variables|Default|Getweapon%20parts))
  (bind _output (Utilities|Array|Get(acopy) _weapon_parts_4 2))
  (bind _output_2 (Utilities|Array|Get(acopy) _weapon_parts_5 4))
  (bind _output_3 (Utilities|Array|Get(acopy) _weapon_parts_2 1))
  (bind _output_4 (Utilities|Array|Get(acopy) _weapon_parts_3))
  (bind _output_5 (Utilities|Array|Get(acopy) _weapon_parts 3))
  (Utilities|FlowControl|Sequence
    (:then_0
      (Utilities|IsValid _output_4
        (:Is%20Valid
          (Components|StaticMesh|SetStaticMesh (Variables|Default|GetFrame_Socket) _output_4)
          (Utilities|FlowControl|Sequence
            (:then_0
              (Utilities|IsValid _output_5
                (:Is%20Valid
                  (Components|StaticMesh|SetStaticMesh (Variables|Default|GetTrigger_Socket) _output_5))))
            (:then_1
              (Utilities|IsValid _output_3
                (:Is%20Valid
                  (Components|StaticMesh|SetStaticMesh (Variables|Default|GetBarrel_Socket) _output_3))))))))
    (:then_1
      (Utilities|IsValid _output
        (:Is%20Valid
          (Components|StaticMesh|SetStaticMesh (Variables|Default|GetMagazine_Socket) _output))))
    (:then_2
      (Utilities|IsValid _output_2
        (:Is%20Valid
          (Components|StaticMesh|SetStaticMesh (Variables|Default|GetSlider_Socket) _output_2))))))

(fn ConstructionScript
  (|CallParentFunction))