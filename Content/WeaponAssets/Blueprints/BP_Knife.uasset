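; BP_Knife is a modular knife weapon that assembles its look from part meshes and a color when play begins.
; It creates a dynamic material for WeaponBase as the grip, waits one tick, then tints its emission with Color.
; Valid WeaponParts entries fill the blade and guard sockets, and the blade gets its own dynamic material with the same emission tint.
; The construction script only calls its parent.
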(event EventBeginPlay
  (bind _weapon_parts (Variables|Default|Getweapon%20parts))
  (bind _blade_socket (Variables|Default|GetBlade_Socket))
  (bind _weapon_parts_2 (Variables|Default|Getweapon%20parts))
  (bind _output (Utilities|Array|Get(acopy) _weapon_parts 1))
  (bind _output_2 (Utilities|Array|Get(acopy) _weapon_parts_2))
  (bind _returnvalue (Rendering|Material|CreateDynamicMaterialInstance (Variables|Default|GetWeaponBase) 0 0 "None" :!class /Script/Engine.PrimitiveComponent))
  (Variables|Default|SetGripMaterial _returnvalue)
  (Utilities|FlowControl|DelayUntilNextTick)
  (Rendering|Material|SetVectorParameterValue (Variables|Default|GetGripMaterial) "EmissionColor" (Variables|Default|GetColor) :!class /Script/Engine.MaterialInstanceDynamic)
  (Utilities|FlowControl|Sequence
    (:then_0
      (Utilities|IsValid _output_2
        (:Is%20Valid
          (Components|StaticMesh|SetStaticMesh _blade_socket _output_2)
          (bind _returnvalue_2 (Rendering|Material|CreateDynamicMaterialInstance _blade_socket 0 0 "None" :!class /Script/Engine.PrimitiveComponent))
          (bind _output_get (Variables|Default|SetBladeMaterial _returnvalue_2))
          (Rendering|Material|SetVectorParameterValue _output_get "EmissionColor" (Variables|Default|GetColor) :!class /Script/Engine.MaterialInstanceDynamic))))
    (:then_1
      (Utilities|IsValid _output
        (:Is%20Valid
          (Components|StaticMesh|SetStaticMesh (Variables|Default|GetGuard_Socket) _output))))))

(fn ConstructionScript
  (|CallParentFunction))