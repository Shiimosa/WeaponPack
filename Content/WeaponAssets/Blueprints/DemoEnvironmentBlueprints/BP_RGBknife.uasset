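; BP_RGBknife is a demo-environment knife whose blade and grip change emissive color over time.
; The construction script creates dynamic material instances for the first material slot of the Blade and Grip components.
; On BeginPlay, the ColoChange timeline plays from the start and writes its color track to the EmissionColor parameter of both instances on every update.
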(event EventBeginPlay
  (bind _newtrack_0 (Timeline|ColoChange PlayFromStart)
    (:Update
      (Rendering|Material|SetVectorParameterValue (Variables|Default|GetMaterial1) "EmissionColor" _newtrack_0 :!class /Script/Engine.MaterialInstanceDynamic)
      (Rendering|Material|SetVectorParameterValue (Variables|Default|GetMaterial2) "EmissionColor" _newtrack_0 :!class /Script/Engine.MaterialInstanceDynamic))))

(fn ConstructionScript
  (bind _returnvalue (Rendering|Material|CreateDynamicMaterialInstance (Variables|Default|GetBlade) 0 0 "None" :!class /Script/Engine.PrimitiveComponent))
  (Variables|Default|SetMaterial1 _returnvalue)
  (bind _returnvalue_2 (Rendering|Material|CreateDynamicMaterialInstance (Variables|Default|GetGrip) 0 0 "None" :!class /Script/Engine.PrimitiveComponent))
  (Variables|Default|SetMaterial2 _returnvalue_2))