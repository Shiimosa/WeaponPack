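; Spawner actor that places one selected weapon or attachment (knife, sword, pistol, scope or muffler) in the level.
; On BeginPlay it switches on ItemToSpawn and spawns the matching Blueprint at the SpawnLocation component's world position.
; Each spawned item receives a reference back to the spawner.
; Weapons also take the emission color, while scopes and mufflers take their chosen variant and update their model.
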(event EventBeginPlay
  (bind _spawnlocation (Variables|Default|GetSpawnLocation))
  (bind _returnvalue (Transformation|GetWorldLocation _spawnlocation))
  (bind _returnvalue_2 (Math|Conversions|ToTransform(Vector) _returnvalue))
  (switch Utilities|FlowControl|Switch|SwitchonE_Items (Variables|ItemSelection|GetItemToSpawn)
    (:NewEnumerator0
      (bind _returnvalue_3 (Game|SpawnActorfromClass "/Game/WeaponAssets/Blueprints/BP_Knife.BP_Knife_C" _returnvalue_2 "Undefined" 0 0))
      (Variables|/Game/WeaponAssets/Blueprints/BP_Weapons.BP_Weapons_C|SetSpawner _returnvalue_3 self)
      (Variables|/Game/WeaponAssets/Blueprints/BP_Knife.BP_Knife_C|SetColor _returnvalue_3 (Variables|WeaponEmissionColor|GetEmissionColor)))
    (:NewEnumerator1
      (bind _returnvalue_4 (Game|SpawnActorfromClass "/Game/WeaponAssets/Blueprints/BP_Sword.BP_Sword_C" _returnvalue_2 "Undefined" 0 0))
      (Variables|/Game/WeaponAssets/Blueprints/BP_Weapons.BP_Weapons_C|SetSpawner _returnvalue_4 self)
      (Variables|/Game/WeaponAssets/Blueprints/BP_Sword.BP_Sword_C|SetColor _returnvalue_4 (Variables|WeaponEmissionColor|GetEmissionColor)))
    (:NewEnumerator2
      (bind _returnvalue_5 (Game|SpawnActorfromClass "/Game/WeaponAssets/Blueprints/BP_Pistol.BP_Pistol_C" _returnvalue_2 "Undefined" 0 0))
      (Variables|/Game/WeaponAssets/Blueprints/BP_Weapons.BP_Weapons_C|SetSpawner _returnvalue_5 self)
      (Variables|/Game/WeaponAssets/Blueprints/BP_Pistol.BP_Pistol_C|SetColor _returnvalue_5 (Variables|WeaponEmissionColor|GetEmissionColor)))
    (:NewEnumerator3
      (bind _returnvalue_6 (Game|SpawnActorfromClass "/Game/WeaponAssets/Blueprints/BP_Scope.BP_Scope_C" _returnvalue_2 "Undefined" 0 0))
      (Variables|/Game/WeaponAssets/Blueprints/BP_GunAttachment.BP_GunAttachment_C|SetSpawner _returnvalue_6 self)
      (Variables|/Game/WeaponAssets/Blueprints/BP_Scope.BP_Scope_C|SetScopeToUse _returnvalue_6 (Math|Conversions|ToInteger(Byte) (Variables|itemselection|GetScopeToSpawn)))
      (Default|SetScopeModel _returnvalue_6))
    (:NewEnumerator4
      (bind _returnvalue_7 (Game|SpawnActorfromClass "/Game/WeaponAssets/Blueprints/BP_Muffler.BP_Muffler_C" _returnvalue_2 "Undefined" 0 0))
      (Variables|/Game/WeaponAssets/Blueprints/BP_GunAttachment.BP_GunAttachment_C|SetSpawner _returnvalue_7 self)
      (Variables|/Game/WeaponAssets/Blueprints/BP_Muffler.BP_Muffler_C|SetMufflerToUse _returnvalue_7 (Math|Conversions|ToInteger(Byte) (Variables|ItemSelection|GetMufflerToSpawn)))
      (Default|SetMufflerModel _returnvalue_7))))

(fn ConstructionScript)